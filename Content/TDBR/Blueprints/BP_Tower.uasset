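; Tower actor that automatically shoots BP_Arrow projectiles at units within its range.
; A looping timer drives detection, taking the first BP_Unit overlapping a sphere sized from Range in the construction script.
; A Serv_ event turns the mesh toward the target and plays a montage scaled by AttackSpeed, blocking attacks until blend-out.
; The montage's "Attack" notify spawns an arrow at a mesh socket, aimed at the target.
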(event `self.ReceiveBeginPlay`
  (`KismetSystemLibrary.K2_SetTimerDelegate` (`|CreateDelegate` :!event `HasRange`) 0.333 true))

(event `Serv_GetUnit`
  (bind _currenttarget (`self.CurrentTarget`)
    (:`then`
      (bind (_returnvalue_roll _returnvalue_pitch _returnvalue_yaw) (`KismetMathLibrary.BreakRotator` (`KismetMathLibrary.FindLookAtRotation` (`self.K2_GetActorLocation`) (`self.K2_GetActorLocation` _currenttarget))))
      (`SceneComponent.K2_SetWorldRotation` (`self.SkeletalMesh`) (`KismetMathLibrary.MakeRotator` 0.0 0.0 (- _returnvalue_yaw 90.0)) false false)
      (bind _returnvalue (`AnimSequenceBase.GetPlayLength` (`self.Montage to Play`)))
      (bind _notifyname (`|PlayMontage` (`self.SkeletalMesh`) (`self.Montage to Play`) (/ (`self.AttackSpeed`) _returnvalue))
        (:`then`
          (set `self.bIsCanAttack` false))
        (:`OnBlendOut`
          (set `self.bIsCanAttack` true))
        (:`OnNotifyBegin`
          (if (== _notifyname "Attack")
            (`self.Shoot`)))))
    (:`else`)))

(event `HasRange`
  (bind _overlappingactors (`PrimitiveComponent.GetOverlappingActors` (`self.SphereDetection`) "/Game/TDBR/Blueprints/BP_Unit.BP_Unit_C"))
  (if (and (`self.bIsCanAttack`) (> (`KismetArrayLibrary.Array_Length` _overlappingactors) 0))
    (set `self.CurrentTarget` (`|GetArrayItem` _overlappingactors))
    (`self.Serv_GetUnit`)))

(event `Shoot`
  (bind _returnvalue (`SceneComponent.GetSocketLocation` (`self.SkeletalMesh`) "LeftWeaponShield"))
  (`|SpawnActorFromClass` "/Game/TDBR/Blueprints/BP_Arrow.BP_Arrow_C" (`KismetMathLibrary.MakeTransform` _returnvalue (`KismetMathLibrary.FindLookAtRotation` _returnvalue (`self.K2_GetActorLocation` (`self.CurrentTarget`)))) "Undefined" "OverrideRootScale" null null))

(fn `OnRep_bIsCanAttack`)

(fn `UserConstructionScript`
  (`SphereComponent.SetSphereRadius` (`self.SphereDetection`) (`self.Range`) true))