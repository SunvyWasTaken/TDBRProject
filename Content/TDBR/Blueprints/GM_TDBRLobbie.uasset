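; Lobby game mode that gathers players and starts the match on L_Map once all are ready.
; PostLogin stores each joining controller and calls DisplayInGame on its PC_Lobbie.
; LaunchTravel checks the IsReady flag of every stored controller, then opens L_Map by object reference with a "servertravel" option, leaving an unused console command node.
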(event `self.K2_PostLogin`
  (params (NewPlayer :type "PlayerController Object Reference"))
  (`KismetArrayLibrary.Array_Add` (`self.ControllerList`) NewPlayer)
  (bind _aspc_lobbie (cast `/Game/TDBR/Blueprints/PC_Lobbie` NewPlayer))
  (`/Game/TDBR/Blueprints/PC_Lobbie.DisplayInGame` _aspc_lobbie))

(event `LaunchTravel`
  (if (`self.CheckIfAllReady`)
    (`GameplayStatics.OpenLevelBySoftObjectPtr` "/Game/TDBR/Map/L_Map.L_Map" false "servertravel")))

(fn `CheckIfAllReady`
  (returns (`Ready?` :type Boolean))
  (for _array_element (`self.ControllerList`)
    (bind _aspc_lobbie (cast `/Game/TDBR/Blueprints/PC_Lobbie` _array_element))
    (if (not (`/Game/TDBR/Blueprints/PC_Lobbie.Is Ready` _aspc_lobbie))
      (return false)))
  (return true))

(fn `UserConstructionScript`)