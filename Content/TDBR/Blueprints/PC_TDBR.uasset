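; PC_TDBR is a player controller that lets the player place BP_Block towers on a grid with the mouse.
; Each tick it traces from the cursor into the world and moves CurrentTower to the hit point, truncated to a 100-unit grid and raised slightly.
; Left-click releases the tower in place, and the next tick spawns a replacement, printing its name.
; The WBP_Interface widget creation is unconnected and never runs.
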(event `self.ReceiveTick`
  (params (DeltaSeconds :type "Float (single-precision)"))
  (bind (_worldlocation _worlddirection) (`self.DeprojectMousePositionToWorld`))
  (bind _outhit (`KismetSystemLibrary.LineTraceSingle` :`Start` _worldlocation :`End` (+ _worldlocation (* _worlddirection 10000000.0)) :`TraceChannel` "TraceTypeQuery1" :`DrawDebugType` "ForDuration"))
  (bind _currenttower (`self.CurrentTower`)
    (:`then`
      (bind _returnvalue (`KismetMathLibrary.FTrunc` (.x (`.Location` (`GameplayStatics.BreakHitResult` _outhit)))))
      (bind _returnvalue_2 (`KismetMathLibrary.FTrunc` (.y (`.Location` (`GameplayStatics.BreakHitResult` _outhit)))))
      (bind _returnvalue_3 (`KismetMathLibrary.MakeVector` (`KismetMathLibrary.Conv_IntToDouble` (- _returnvalue (mod _returnvalue 100))) (`KismetMathLibrary.Conv_IntToDouble` (- _returnvalue_2 (mod _returnvalue_2 100))) (- (.z (`.Location` (`GameplayStatics.BreakHitResult` _outhit))) -52.0)))
      (`self.K2_SetActorLocation` _currenttower _returnvalue_3 false false))
    (:`else`
      (bind _returnvalue_4 (`|SpawnActorFromClass` "/Game/TDBR/Blueprints/BP_Block.BP_Block_C" (`KismetMathLibrary.MakeTransform` _returnvalue_3) "Undefined" "OverrideRootScale" null null))
      (bind _output_get (set `self.CurrentTower` _returnvalue_4))
      (`KismetSystemLibrary.PrintString` (`KismetSystemLibrary.GetDisplayName` _output_get) true true (struct :`R` 1.0 :`G` 0.036994 :`A` 1.0)))))

(event `Key|LeftMouseButton`
  (params (Key :type "Key Structure"))
  (:`Pressed`
    (set `self.CurrentTower` null)))

(fn `UserConstructionScript`)