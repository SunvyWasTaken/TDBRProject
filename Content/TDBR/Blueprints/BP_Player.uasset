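; BP_Player is the player pawn, providing directional movement and mouse-wheel camera zoom.
; Forward and Right axes add movement input along the Scene component's forward and right vectors.
; Wheel presses step a clamped ZoomAlpha that blends the target field of view between wide and narrow.
; A looping timer event moves the camera FOV toward that target at constant speed, clearing itself once it settles.
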(event `InputAxis|Forward`
  (params (AxisValue :type "Float (single-precision)"))
  (`self.AddMovementInput` (`SceneComponent.GetForwardVector` (`self.Scene`)) AxisValue))

(event `Key|MouseScrollUp`
  (params (Key :type "Key Structure"))
  (bind _returnvalue (+ (`self.ZoomAlpha`) 0.2))
  (:`Pressed`
    (set `self.ZoomAlpha` (`KismetMathLibrary.SelectFloat` 1.0 _returnvalue (>= _returnvalue 1.0)))
    (bind _returnvalue_2 (`KismetSystemLibrary.K2_SetTimerDelegate` (delegate `ZoomEvent`) 0.033333 true :!label _label))))

(event `ZoomEvent`
  (bind _camera (`self.Camera`))
  (bind _fieldofview (`CameraComponent.FieldOfView` _camera))
  (bind _returnvalue (`KismetMathLibrary.FInterpTo_Constant` _fieldofview (`KismetMathLibrary.Lerp` 90.0 40.0 (`self.ZoomAlpha`)) 0.033333 50.0))
  (`CameraComponent.SetFieldOfView` _camera _returnvalue)
  (if (== _returnvalue _fieldofview)
    (`KismetSystemLibrary.K2_ClearAndInvalidateTimerHandle` (stale `Key|MouseScrollUp` _returnvalue_2))))

(event `InputAxis|Right`
  (params (AxisValue :type "Float (single-precision)"))
  (`self.AddMovementInput` (`SceneComponent.GetRightVector` (`self.Scene`)) AxisValue))

(event `Key|MouseScrollDown`
  (params (Key :type "Key Structure"))
  (bind _returnvalue (- (`self.ZoomAlpha`) 0.2))
  (:`Pressed`
    (set `self.ZoomAlpha` (`KismetMathLibrary.SelectFloat` 0.0 _returnvalue (<= _returnvalue 0.0)))
    (goto _label)))

(fn `UserConstructionScript`)