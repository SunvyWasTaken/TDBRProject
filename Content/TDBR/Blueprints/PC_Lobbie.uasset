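; Lobby player controller that shows the lobby UI and handles the player's ready state.
; DisplayInGame creates the WBP_Lobbie widget, binds its SetReady dispatcher, adds it to the viewport and switches input to UI only.
; SetReady stores IsReady and calls LaunchTravel on GM_TDBRLobbie whatever the value, printing a debug string if the game mode cast fails.
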(event `DisplayInGame`
  (bind _returnvalue (`|CreateWidget` "/Game/TDBR/Widget/WBP_Lobbie.WBP_Lobbie_C"))
  (add `/Game/TDBR/Widget/WBP_Lobbie.SetReady` _returnvalue (`|CreateDelegate` :!event `SetReady`))
  (`UserWidget.AddToViewport` _returnvalue 0)
  (`WidgetBlueprintLibrary.SetInputMode_UIOnlyEx` self _returnvalue))

(event `SetReady`
  (params (IsReady :type Boolean))
  (set `self.Is Ready` IsReady)
  (bind _asgm_tdbrlobbie (cast `/Game/TDBR/Blueprints/GM_TDBRLobbie` (`GameplayStatics.GetGameMode`))
    (:`then`
      (`/Game/TDBR/Blueprints/GM_TDBRLobbie.LaunchTravel` _asgm_tdbrlobbie))
    (:`CastFailed`
      (`KismetSystemLibrary.PrintString` "Hello"))))

(fn `UserConstructionScript`)