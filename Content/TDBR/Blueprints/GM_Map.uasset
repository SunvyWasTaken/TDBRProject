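; Game mode for a TDBR map that registers joining players and can pay money to all of them.
; BeginPlay destroys the session of the first player controller.
; PostLogin has each PC_TDBR draw its UI, adds it to PlayerList and starts a one-second looping timer, so every login creates another timer.
; Serv_AddMoney gives one money to every listed controller, likely as that timer's callback, though the binding is not shown.
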(event `self.ReceiveBeginPlay`
  (`DestroySessionCallbackProxy.DestroySession` (`GameplayStatics.GetPlayerController` 0)))

(event `self.K2_PostLogin`
  (params (NewPlayer :type "PlayerController Object Reference"))
  (bind _aspc_tdbr (cast `/Game/TDBR/Blueprints/PC_TDBR` NewPlayer))
  (`/Game/TDBR/Blueprints/PC_TDBR.Client_DrawUI` _aspc_tdbr)
  (bind _aspc_tdbr_2 (cast `/Game/TDBR/Blueprints/PC_TDBR` NewPlayer))
  (`self.AddPCOnList` _aspc_tdbr_2)
  (`KismetSystemLibrary.K2_SetTimerDelegate` (`|CreateDelegate` :!event `Serv_AddMoney`) 1.0 true))

(event `AddPCOnList`
  (params (PlayerController :type "/Game/TDBR/Blueprints/PC_TDBR Object Reference"))
  (`KismetArrayLibrary.Array_Add` (`self.PlayerList`) PlayerController))

(event `Serv_AddMoney`
  (for _array_element (`self.PlayerList`)
    (`/Game/TDBR/Blueprints/PC_TDBR.AddMoney` _array_element 1)))

(fn `UserConstructionScript`)