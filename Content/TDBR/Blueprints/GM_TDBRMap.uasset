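; Game mode for the TDBR map that registers joining players and provides logic for granting them money.
; On login it has the client draw its UI, lists the controller, assigns a player number as a surface-type enum from the player count, and starts a looping one-second server timer on each login.
; Serv_AddMoney gives every listed player one money, while SpawnUnitToOtherr loops over players but spawns nothing yet.
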(event `self.ReceiveBeginPlay`)

(event `self.K2_PostLogin`
  (params (NewPlayer :type "PlayerController Object Reference"))
  (bind _aspc_tdbr (cast `/Game/TDBR/Blueprints/PC_TDBR` NewPlayer))
  (`/Game/TDBR/Blueprints/PC_TDBR.Client_DrawUI` _aspc_tdbr)
  (`self.AddPCOnList` _aspc_tdbr)
  (bind _returnvalue (`self.GetNumPlayers`))
  (`KismetSystemLibrary.PrintString` (`KismetStringLibrary.Conv_IntToString` _returnvalue))
  (set `/Game/TDBR/Blueprints/PC_TDBR.PlayerNbr` (select `int` _returnvalue :`0` "SurfaceType_Default" :`1` "SurfaceType1" :`2` "SurfaceType2" :`3` "SurfaceType3" :`4` "SurfaceType4" :!type "EPhysicalSurface Enum") _aspc_tdbr)
  (if (`KismetSystemLibrary.IsServer`)
    (`KismetSystemLibrary.K2_SetTimerDelegate` (`|CreateDelegate` :!event `Serv_AddMoney`) 1.0 true)))

(event `AddPCOnList`
  (params (PlayerController :type "/Game/TDBR/Blueprints/PC_TDBR Object Reference"))
  (`KismetArrayLibrary.Array_Add` (`self.PlayerList`) PlayerController))

(event `Serv_AddMoney`
  (for _array_element (`self.PlayerList`)
    (`/Game/TDBR/Blueprints/PC_TDBR.AddMoney` _array_element 1)))

(event `SpawnUnitToOtherr`
  (params (Player :type "Object Object Reference") (UnitToSpawn :type "Actor Class Reference"))
  (for _array_element (`self.PlayerList`)
    (if (!= _array_element Player)
      _)))

(fn `UserConstructionScript`)