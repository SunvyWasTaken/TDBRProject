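; BP_Unit is a killable AI-moved unit that heads for a target actor, noted as the Base, and pays gold when killed.
; On BeginPlay it fills its health and uses AIMoveTo toward the current entry in its Target array.
; AnyDamage stores the instigator, lowers health and updates the WBP_HealthBar widget.
; At zero health it awards GoldValue to the instigating PC_TDBR and destroys itself, but only if that cast succeeds.
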(event `self.ReceiveBeginPlay`
  ;[1 1 1] Define HP
  (set `self.CurrentHealth` (`self.MaxHealth`))
  (`self.StartMoving`))

(event `Regen`
  (set `self.CurrentHealth` (`self.MaxHealth`)))

(event `/Game/TDBR/Blueprints/BPI_Damageable.Hit`
  (params (DamageInput :type Integer))
  (set `self.CurrentHealth` (- (`self.CurrentHealth`) DamageInput)))

(event `TestPath`
  (for _array_element (`NavigationPath.PathPoints` (`AIBlueprintHelperLibrary.GetCurrentPath` (`AIBlueprintHelperLibrary.GetAIController` self)))
    (`KismetSystemLibrary.PrintString` (`KismetStringLibrary.Conv_VectorToString` _array_element))))

(event `StartMoving`
  (bind _target (`self.Target`))
  ;[1 1 1] Move the unit to the Base
  (if (> (`KismetArrayLibrary.Array_Length` _target) 0)
    (`|AIMoveTo` self (0.0 0.0 0.0) (`|GetArrayItem` _target (`self.CurrentTargetIndex`)) 5.0 true)))

(event `self.ReceiveAnyDamage`
  (params (Damage :type "Float (single-precision)") (DamageType :type "DamageType Object Reference") (InstigatedBy :type "Controller Object Reference") (DamageCauser :type "Actor Object Reference"))
  (set `self.Instigated By` InstigatedBy)
  (`self.ApplyOnAll` Damage))

(event `ApplyOnAll`
  (params (A :type "Float (double-precision)"))
  ;[1 1 1] Calculate the damage the unit received
  (set `self.CurrentHealth` (- (`self.CurrentHealth`) (`KismetMathLibrary.FTrunc` A)))
  (bind _aswbp_health_bar (cast `/Game/TDBR/Widget/WBP_HealthBar` (`WidgetComponent.GetWidget` (`self.Widget`)))
    (:`then`
      (set `/Game/TDBR/Widget/WBP_HealthBar.HealthPercent` (/ (`KismetMathLibrary.Conv_IntToDouble` (`self.CurrentHealth`)) (`KismetMathLibrary.Conv_IntToDouble` (`self.MaxHealth`))) _aswbp_health_bar))
    (:`CastFailed`
      _))
  (if (<= (`self.CurrentHealth`) 0)
    (`self.UnitDie`)))

(event `UnitDie`
  ;[1 1 1] Destroy the Unit On the Server
  (bind _aspc_tdbr (cast `/Game/TDBR/Blueprints/PC_TDBR` (`self.Instigated By`)))
  (`/Game/TDBR/Blueprints/PC_TDBR.AddMoney` _aspc_tdbr (`self.GoldValue`))
  (`self.K2_DestroyActor`))

(fn `UserConstructionScript`)